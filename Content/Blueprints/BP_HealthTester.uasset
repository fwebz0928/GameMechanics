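; BP_HealthTester is a test actor that continuously damages or heals the player character while it overlaps the actor's Cube.
; Begin overlap caches the BP_FirstPersonCharacter and opens a Gate, and end overlap closes it.
; While the Gate is open, Tick calls DamageHealth or Heal on the character's health component, chosen by a boolean.
; The fixed amount applies every frame without delta-time scaling, so the rate depends on framerate.
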(event `self.ReceiveTick`
  (params (DeltaSeconds :type "Float (single-precision)"))
  (`/Engine/EditorBlueprintResources/StandardMacros.Gate` true :!label _label
    (:`Exit`
      (if (`self.DamageHealth`)
        (bind _returnvalue (`GameMechanicsCharacter.GetHealthComponent` (stale `self.Cube.OnComponentBeginOverlap` _asbp_first_person_character)))
        (`HealthComponent.DamageHealth` _returnvalue 1.0)
        (else
          (`HealthComponent.Heal` _returnvalue 1.0))))))

(event `self.Cube.OnComponentBeginOverlap`
  (params (OverlappedComponent :type "PrimitiveComponent Object Reference") (OtherActor :type "Actor Object Reference") (OtherComp :type "PrimitiveComponent Object Reference") (OtherBodyIndex :type Integer) (bFromSweep :type Boolean) (SweepResult :type "HitResult Structure (by ref)"))
  (bind _returnvalue (`GameplayStatics.GetPlayerCharacter` 0))
  (if (== OtherActor _returnvalue)
    (bind _asbp_first_person_character (cast `/Game/Blueprints/BP_FirstPersonCharacter` _returnvalue))
    (goto _label :!via `Open`)))

(event `self.Cube.OnComponentEndOverlap`
  (params (OverlappedComponent :type "PrimitiveComponent Object Reference") (OtherActor :type "Actor Object Reference") (OtherComp :type "PrimitiveComponent Object Reference") (OtherBodyIndex :type Integer))
  (if (== OtherActor (`GameplayStatics.GetPlayerCharacter` 0))
    (goto _label :!via `Close`)))

(fn `UserConstructionScript`)