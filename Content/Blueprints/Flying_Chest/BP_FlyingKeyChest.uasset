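; Flying key chest minigame Blueprint that activates when a BP_FlyingKey reaches its trigger, letting the player smack the key with Space or exit with K.
; The key mesh eases to random points in an area, pausing randomly between moves.
; SmackTrigger overlaps track whether the key is in the hit zone.
; Opening hides the key, swings the doors via a timeline, then marks the chest beaten.
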(event `Key|SpaceBar`
  (params (Key :type "Key Structure"))
  ;[1 1 1] Inputs
  (:`Pressed`
    (`self.SmackKey`)))

(event `Key|K`
  (params (Key :type "Key Structure"))
  ;[1 1 1] Inputs
  (:`Pressed`
    (`self.ExitChest`)))

(event `self.TriggerBox.OnComponentBeginOverlap`
  (params (OverlappedComponent :type "PrimitiveComponent Object Reference") (OtherActor :type "Actor Object Reference") (OtherComp :type "PrimitiveComponent Object Reference") (OtherBodyIndex :type Integer) (bFromSweep :type Boolean) (SweepResult :type "HitResult Structure (by ref)"))
  ;[1 0.3379 0.4783] Called whern the flying key actor reaches this key chest
  (bind _asbp_flying_key (cast `/Game/Blueprints/Flying_Chest/BP_FlyingKey` OtherActor))
  (`self.KeyAtLocation` _asbp_flying_key))

(event `self.MoveKeyToPositionOnSide`
  ;[1 1 1] Move the component to the actual positioon smoothly
  (`KismetSystemLibrary.MoveComponentTo` (`self.KeyMesh`) (`self.GetRandomPointInArea`) (struct) true true 2.0 :!label _label)
  (`KismetSystemLibrary.Delay` (`KismetMathLibrary.RandomFloatInRange` 1.0 3.0))
  (`self.MovementTimelineCallback` 0.0))

(event `self.StopMovingKey`
  ;[1 1 1] Move the component to the actual positioon smoothly
  (goto _label :!via `Stop`))

(event `self.SmackTrigger.OnComponentBeginOverlap`
  (params (OverlappedComponent :type "PrimitiveComponent Object Reference") (OtherActor :type "Actor Object Reference") (OtherComp :type "PrimitiveComponent Object Reference") (OtherBodyIndex :type Integer) (bFromSweep :type Boolean) (SweepResult :type "HitResult Structure (by ref)"))
  ;[1 0.8803 0.2678] Overlaps to detect when the key mesh is actually in the zone
  (`self.DetectKeyInZone` OtherComp true))

(event `self.OpenDoors`
  ;[1 1 1] Swing the door open
  (`SceneComponent.SetVisibility` (`self.KeyMesh`) false false)
  (bind (_direction _value) (`Timeline|RotateDoors`)
    (:`Update`
      (`self.OpenDoorsTimeline` _value))
    (:`Finished`
      (`self.ChestBeaten`))))

(event `self.SmackTrigger.OnComponentEndOverlap`
  (params (OverlappedComponent :type "PrimitiveComponent Object Reference") (OtherActor :type "Actor Object Reference") (OtherComp :type "PrimitiveComponent Object Reference") (OtherBodyIndex :type Integer))
  ;[1 0.8803 0.2678] Overlaps to detect when the key mesh is actually in the zone
  (`self.DetectKeyInZone` OtherComp))

(fn `BP_FlyingKeyChest_AutoGenFunc`)

(fn `UserConstructionScript`)